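; BP_DamageCylinder is an interactable actor with a moving cylinder; despite its name, it contains no damage logic.
; A looping timer set on BeginPlay fires MoveInSeconds, which calls two move functions back to back with no delay.
; Each issues a timed MoveComponentTo toward opposite diagonal XY offsets at fixed height.
; Targets derive from the cylinder's world location but are passed as relative locations.
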(event `MoveInSeconds`
  (bind _cylinder (`self.Cylinder`))
  (bind _cylinder_2 (`self.Cylinder`))
  (bind (_returnvalue_x _returnvalue_y) (`KismetMathLibrary.BreakVector` (`SceneComponent.K2_GetComponentLocation` _cylinder)))
  (bind (_returnvalue_x_2 _returnvalue_y_2) (`KismetMathLibrary.BreakVector` (`SceneComponent.K2_GetComponentLocation` _cylinder_2)))
  (`KismetSystemLibrary.MoveComponentTo` _cylinder_2 (`KismetMathLibrary.MakeVector` (+ _returnvalue_x_2 50.0) (+ _returnvalue_y_2 50.0) 40.0) (struct) false false 0.8)
  (`KismetSystemLibrary.MoveComponentTo` _cylinder (`KismetMathLibrary.MakeVector` (+ _returnvalue_x -50.0) (+ _returnvalue_y -50.0) 40.0) (struct) false false 0.8))

(event `self.ReceiveBeginPlay`
  (`parent.ReceiveBeginPlay`)
  (`KismetSystemLibrary.K2_SetTimer` null "MoveInSeconds" 1.7 true))

(fn `UserConstructionScript`
  (`parent.UserConstructionScript`))