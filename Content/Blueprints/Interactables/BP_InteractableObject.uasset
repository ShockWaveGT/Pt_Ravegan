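; Interactable object actor that hides itself when the third-person character reports a collision with it.
; On BeginPlay it gets the player character and binds to its interactable-collision and game-over events.
; A matching collision hides the actor and teleports it below the world origin, unless CannotBeHidden is set.
; The game-over handler, despite its name ReturnObjects, also just hides the actor.
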(event `CheckCollision`
  (params (InteractableObject :type "/Game/Blueprints/Interactables/BP_InteractableObject Object Reference"))
  (if (== InteractableObject self)
    (if (not (`self.CannotBeHidden`))
      (`self.SetActorHiddenInGame` self true)
      (`self.K2_TeleportTo` :`self` self :`DestLocation` (0.0 0.0 -1000.0)))))

(event `self.ReceiveBeginPlay`
  (bind _asbp_third_person_character (cast `/Game/Blueprints/BP_ThirdPersonCharacter` (`GameplayStatics.GetPlayerCharacter` 0)))
  (add `/Game/Blueprints/BP_ThirdPersonCharacter.CollisionWithInteractable` _asbp_third_person_character (delegate `CheckCollision`))
  (add `/Game/Blueprints/BP_ThirdPersonCharacter.GameOver` _asbp_third_person_character (delegate `ReturnObjects`)))

(event `ReturnObjects`
  (`self.SetActorHiddenInGame` true))

(fn `UserConstructionScript`)